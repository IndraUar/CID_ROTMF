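; Artifact_P1 is a collectible artifact that acts as a save checkpoint when the third-person character hits it.
; The first hit writes a Lever_Save to slot "Artifact_P1" with the artifact's transform as player position, timer values, an artifact flag, and the first found lever switcher's state and two linked door transforms.
; It then prints a confirmation and destroys itself.
; Load and lever-restore logic exists but never runs.
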(event Collision|EventHit
  (params (MyComp :type Primitive%20Component%20Object%20Reference) (Other :type Actor%20Object%20Reference) (OtherComp :type Primitive%20Component%20Object%20Reference) (bSelfMoved :type Boolean) (HitLocation :type Vector :default "0, 0, 0") (HitNormal :type Vector :default "0, 0, 0") (NormalImpulse :type Vector :default "0, 0, 0") (Hit :type Hit%20Result%20Structure%20%28by%20ref%29))
  (bind _output_get (Variables|Default|SetOther Other))
  (Utilities|Casting|CastToBP_ThirdPersonCharacter _output_get)
  (Utilities|FlowControl|DoOnce false
    (:Completed
      (bind _returnvalue (SaveGame|CreateSaveGameObject "/Game/BluePrint/Save_And_Load/Lever_Save.Lever_Save_C"))
      (Variables|/Game/BluePrint/Save_And_Load/Lever_Save.Lever_Save_C|SetPlayerPosition _returnvalue (Transformation|GetActorTransform))
      (bind _returnvalue_2 (Actor|GetActorOfClass "/Game/BluePrint/Pull_Lever/BP_LeverSwitcher.BP_LeverSwitcher_C"))
      (Variables|/Game/BluePrint/Save_And_Load/Lever_Save.Lever_Save_C|SetMainDoor_Lever _returnvalue (Variables|/Game/BluePrint/Pull_Lever/BP_LeverSwitcher.BP_LeverSwitcher_C|GetOn _returnvalue_2))
      (Variables|/Game/BluePrint/Save_And_Load/Lever_Save.Lever_Save_C|SetTimer_Second _returnvalue (Variables|Default|GetInitialSecond))
      (Variables|/Game/BluePrint/Save_And_Load/Lever_Save.Lever_Save_C|SetTimer_Minute _returnvalue (Variables|Default|GetInitialMinute))
      (Variables|/Game/BluePrint/Save_And_Load/Lever_Save.Lever_Save_C|SetArtifact_P1 _returnvalue true)
      (Variables|/Game/BluePrint/Save_And_Load/Lever_Save.Lever_Save_C|SetTestDoor_1 _returnvalue (Transformation|GetActorTransform (Variables|/Game/BluePrint/Pull_Lever/BP_LeverSwitcher.BP_LeverSwitcher_C|GetLinkedObject _returnvalue_2)))
      (Variables|/Game/BluePrint/Save_And_Load/Lever_Save.Lever_Save_C|SetTestDoor_2 _returnvalue (Transformation|GetActorTransform (Variables|/Game/BluePrint/Pull_Lever/BP_LeverSwitcher.BP_LeverSwitcher_C|GetLinkedObject_2 _returnvalue_2)))
      (SaveGame|SaveGametoSlot _returnvalue "Artifact_P1")
      (Variables|Default|SetAs%20Lever%20Save _returnvalue)
      (Development|PrintString "Saved")
      (Actor|DestroyActor))))

(fn ConstructionScript)