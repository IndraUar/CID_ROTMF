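; BP_Artifact_P1 is a pickup artifact that acts as a one-time save checkpoint when hit by the third-person character.
; On that hit it creates a Lever_Save object holding its own transform as the player position, lever and artifact flags, and timer values.
; It writes this to the "Artifact_P1" slot, then destroys itself.
; Leftover unconnected nodes sketch loading and lever or door saving, but never run.
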(event Collision|EventHit
  (params (MyComp :type Primitive%20Component%20Object%20Reference) (Other :type Actor%20Object%20Reference) (OtherComp :type Primitive%20Component%20Object%20Reference) (bSelfMoved :type Boolean) (HitLocation :type Vector :default "0, 0, 0") (HitNormal :type Vector :default "0, 0, 0") (NormalImpulse :type Vector :default "0, 0, 0") (Hit :type Hit%20Result%20Structure%20%28by%20ref%29))
  (bind _output_get (Variables|Default|SetOther Other))
  (Utilities|Casting|CastToBP_ThirdPersonCharacter _output_get)
  (Utilities|FlowControl|DoOnce false
    (:Completed
      (bind _returnvalue (SaveGame|CreateSaveGameObject "/Game/BluePrint/Save_And_Load/Lever_Save.Lever_Save_C"))
      (Variables|/Game/BluePrint/Save_And_Load/Lever_Save.Lever_Save_C|SetPlayerPosition _returnvalue (Transformation|GetActorTransform))
      (Variables|/Game/BluePrint/Save_And_Load/Lever_Save.Lever_Save_C|SetP1_Lever_Disable _returnvalue true)
      (Variables|/Game/BluePrint/Save_And_Load/Lever_Save.Lever_Save_C|SetArtifact_P1 _returnvalue true)
      (Variables|/Game/BluePrint/Save_And_Load/Lever_Save.Lever_Save_C|SetTimer_Second _returnvalue (Variables|Default|GetInitialSecond))
      (Variables|/Game/BluePrint/Save_And_Load/Lever_Save.Lever_Save_C|SetTimer_Minute _returnvalue (Variables|Default|GetInitialMinute))
      (SaveGame|SaveGametoSlot _returnvalue "Artifact_P1")
      (Variables|Default|SetAs%20Lever%20Save _returnvalue)
      (Development|PrintString "Saved")
      (Actor|DestroyActor))))

(fn ConstructionScript)