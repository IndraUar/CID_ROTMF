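; Lever switch that drives up to two linked Door_Blue_V1 doors as its handle is pulled back and forth.
; Tick reads the handle's pitch in actor-local space and updates On whenever its sign flips.
; Each change advances a FlipFlop per door, alternating Lift and Lower, with Door1Lift and Door2Lift choosing which comes first.
; The door action follows the toggle count rather than the value of On.
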(event EventTick
  (params (DeltaSeconds :type Float%20%28single-precision%29))
  (bind _returnvalue (Transformation|GetActorTransform))
  (bind _handle (Variables|Default|GetHandle))
  (bind _returnvalue_2 (Transformation|GetWorldRotation _handle))
  (bind _returnvalue_3 (Math|Transform|InverseTransformRotation _returnvalue _returnvalue_2))
  (bind _returnvalue_4 (< (.pitch _returnvalue_3) 0.0))
  (if (!= (Variables|Default|GetOn) _returnvalue_4)
    (Variables|Default|SetOn _returnvalue_4)
    (Utilities|FlowControl|Sequence
      (:then_0
        (if (Variables|Default|GetDoor_1_Lift)
          (Utilities|FlowControl|FlipFlop
            (:A
              (bind _asdoor_blue_v1 (Utilities|Casting|CastToDoor_Blue_V1 (Variables|Default|GetLinkedObject)))
              (Default|Lift _asdoor_blue_v1))
            (:B
              (bind _asdoor_blue_v1_2 (Utilities|Casting|CastToDoor_Blue_V1 (Variables|Default|GetLinkedObject)))
              (Default|Lower _asdoor_blue_v1_2)))
          (else
            (Utilities|FlowControl|FlipFlop
              (:A
                (bind _asdoor_blue_v1_3 (Utilities|Casting|CastToDoor_Blue_V1 (Variables|Default|GetLinkedObject)))
                (Default|Lower _asdoor_blue_v1_3))
              (:B
                (bind _asdoor_blue_v1_4 (Utilities|Casting|CastToDoor_Blue_V1 (Variables|Default|GetLinkedObject)))
                (Default|Lift _asdoor_blue_v1_4))))))
      (:then_1
        (if (Variables|Default|GetDoor_2_Lift)
          (Utilities|FlowControl|FlipFlop
            (:A
              (bind _asdoor_blue_v1_5 (Utilities|Casting|CastToDoor_Blue_V1 (Variables|Default|GetLinkedObject_2)))
              (Default|Lift _asdoor_blue_v1_5))
            (:B
              (bind _asdoor_blue_v1_6 (Utilities|Casting|CastToDoor_Blue_V1 (Variables|Default|GetLinkedObject_2)))
              (Default|Lower _asdoor_blue_v1_6)))
          (else
            (Utilities|FlowControl|FlipFlop
              (:A
                (bind _asdoor_blue_v1_7 (Utilities|Casting|CastToDoor_Blue_V1 (Variables|Default|GetLinkedObject_2)))
                (Default|Lower _asdoor_blue_v1_7))
              (:B
                (bind _asdoor_blue_v1_8 (Utilities|Casting|CastToDoor_Blue_V1 (Variables|Default|GetLinkedObject_2)))
                (Default|Lift _asdoor_blue_v1_8)))))))))

(fn ConstructionScript)