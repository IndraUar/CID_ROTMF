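; Blue lever switch that moves two Door_Blue actors and plays a short camera cutaway to show the result.
; Tick compares the handle's actor-relative pitch to a threshold and fires whenever the On state flips.
; Either flip calls Lift on ToLift and Lower on ToLower, then delays step the view through BlueCam1, BlueCam2 and the player.
; Cinematic mode is enabled at the first camera and released at the second.
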(event EventBeginPlay)

(event EventTick
  (params (DeltaSeconds :type Float%20%28single-precision%29))
  (bind _returnvalue (Transformation|GetActorTransform))
  (bind _returnvalue_2 (Game|GetPlayerController 0))
  (bind _returnvalue_3 (Game|GetPlayerController 0))
  (bind _returnvalue_4 (Game|GetPlayerController 0))
  (bind _handle (Variables|Default|GetHandle))
  (bind _returnvalue_5 (Transformation|GetWorldRotation _handle))
  (bind _returnvalue_6 (Math|Transform|InverseTransformRotation _returnvalue _returnvalue_5))
  (bind _returnvalue_7 (> (.pitch _returnvalue_6) 1.0))
  (if (!= (Variables|Default|GetOn) _returnvalue_7)
    (Variables|Default|SetOn _returnvalue_7)
    (Utilities|FlowControl|Sequence
      (:then_0
        (bind _asdoor_blue (Utilities|Casting|CastToDoor_Blue (Variables|Default|GetToLift)))
        (Default|Lift _asdoor_blue)
        (Development|PrintString "Lift"))
      (:then_1
        (bind _asdoor_blue_2 (Utilities|Casting|CastToDoor_Blue (Variables|Default|GetToLower)))
        (Default|Lower _asdoor_blue_2)
        ;[1 1 1] Cam Switch
        (Utilities|FlowControl|Delay 1.0)
        (Game|Player|SetViewTargetwithBlend _returnvalue_2 (Variables|Default|GetBlueCam1) 0.0 "VTBlend_Linear" 0.0 false)
        (Class|PlayerController|SetCinematicMode _returnvalue_2 true true true true true)
        (Utilities|FlowControl|Delay 2.0)
        (Game|Player|SetViewTargetwithBlend _returnvalue_4 (Variables|Default|GetBlueCam2) 0.0 "VTBlend_Linear" 0.0 false)
        (Class|PlayerController|SetCinematicMode _returnvalue_4 false true true true true)
        (Utilities|FlowControl|Delay 2.0)
        (Game|Player|SetViewTargetwithBlend _returnvalue_3 (Game|GetPlayerCharacter 0) 0.0 "VTBlend_Linear" 0.0 false)
        (Class|PlayerController|SetCinematicMode _returnvalue_3 false true true true true)))))

(fn ConstructionScript)