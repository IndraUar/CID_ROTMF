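; BP_LeverSwitcher_White is a lever switch that operates two white doors and shows a brief camera cut.
; Tick checks the Handle's pitch in actor space against a threshold and reacts whenever that state flips.
; Either flip calls Lift on ToLift and Lower on ToLower, both cast to Door_White.
; After lowering, delays time a view switch to WhiteCam1 in cinematic mode, then back to the player.
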(event EventBeginPlay)

(event Collision|EventActorBeginOverlap
  (params (OtherActor :type Actor%20Object%20Reference)))

(event EventTick
  (params (DeltaSeconds :type Float%20%28single-precision%29))
  (bind _returnvalue (Transformation|GetActorTransform))
  (bind _returnvalue_2 (Game|GetPlayerController 0))
  (bind _returnvalue_3 (Game|GetPlayerController 0))
  (bind _handle (Variables|Default|GetHandle))
  (bind _returnvalue_4 (Transformation|GetWorldRotation _handle))
  (bind _returnvalue_5 (Math|Transform|InverseTransformRotation _returnvalue _returnvalue_4))
  (bind _returnvalue_6 (> (.pitch _returnvalue_5) 1.0))
  (if (!= (Variables|Default|GetOn) _returnvalue_6)
    (Variables|Default|SetOn _returnvalue_6)
    (Utilities|FlowControl|Sequence
      (:then_0
        (bind _asdoor_white (Utilities|Casting|CastToDoor_White (Variables|Default|GetToLift)))
        (Default|Lift _asdoor_white)
        (Development|PrintString "Lift"))
      (:then_1
        (bind _asdoor_white_2 (Utilities|Casting|CastToDoor_White (Variables|Default|GetToLower)))
        (Default|Lower _asdoor_white_2)
        ;[1 1 1] Cam Switch
        (Utilities|FlowControl|Delay 1.0)
        (Game|Player|SetViewTargetwithBlend _returnvalue_2 (Variables|Default|GetWhiteCam1) 0.0 "VTBlend_Linear" 0.0 false)
        (Class|PlayerController|SetCinematicMode _returnvalue_2 true true true true true)
        (Utilities|FlowControl|Delay 2.0)
        (Game|Player|SetViewTargetwithBlend _returnvalue_3 (Game|GetPlayerCharacter 0) 0.0 "VTBlend_Linear" 0.0 false)
        (Class|PlayerController|SetCinematicMode _returnvalue_3 false true true true true)))))

(fn ConstructionScript)