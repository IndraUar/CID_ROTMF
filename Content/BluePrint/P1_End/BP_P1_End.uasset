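; BP_P1_End is an exit trigger that records the P1 escape once the player's artifact is saved.
; Tick reloads the Artifact_P1 save every frame and opens or closes a gate from its ArtifactP1 flag, printing a debug message if no save exists.
; Any actor overlap passing the open gate sets P1Escape on that loaded Lever_Save and writes it back to the slot.
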(event Collision|EventActorBeginOverlap
  (params (OtherActor :type Actor%20Object%20Reference))
  (Utilities|FlowControl|Gate true
    (:Exit
      (if true
        (Variables|/Game/BluePrint/Save_And_Load/Lever_Save.Lever_Save_C|SetP1_Escape (stale EventTick _aslever_save) true)
        (SaveGame|SaveGametoSlot (stale EventTick _aslever_save) "Artifact_P1")
        (Development|PrintString "Saved_Escape")))))

(event EventTick
  (params (DeltaSeconds :type Float%20%28single-precision%29))
  (bind _returnvalue (SaveGame|DoesSaveGameExist "Artifact_P1"))
  (if _returnvalue
    (bind _returnvalue_2 (SaveGame|LoadGamefromSlot "Artifact_P1"))
    (bind _aslever_save (Utilities|Casting|CastToLever_Save _returnvalue_2))
    (if (Variables|/Game/BluePrint/Save_And_Load/Lever_Save.Lever_Save_C|GetArtifact_P1 _aslever_save)
      (Utilities|FlowControl|Gate true) ; enters at Open
      (else
        (Utilities|FlowControl|Gate true) ; enters at Close
      ))
    (else
      (Utilities|FlowControl|DoOnce false
        (:Completed
          (Development|PrintString "No Save(BP End)"))))))

(fn ConstructionScript)