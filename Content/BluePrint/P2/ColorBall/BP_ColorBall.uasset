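; BP_ColorBall is a ball actor that switches between a red and a blue material.
; BeginPlay derives IsRed from the static mesh's starting material, and Tick wakes the mesh's rigid body every frame so its physics does not sleep.
; ChangeColor swaps the material and flips IsRed, also mirroring the state in IsRedInt, which BeginPlay leaves untouched.
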(event EventBeginPlay
  (if (== (Rendering|Material|GetMaterial (Variables|Debug|GetStaticMeshComponent) 0) (Variables|Default|GetMat_Red))
    (Variables|Default|SetIsRed true)
    (else
      (Variables|Default|SetIsRed false))))

(event EventTick
  (params (DeltaSeconds :type Float%20%28single-precision%29))
  (Class|PrimitiveComponent|WakeRigidBody (Variables|Debug|GetStaticMeshComponent) "None"))

(fn ConstructionScript)

(fn ChangeColor
  (if (Variables|Default|GetIsRed)
    (Rendering|Material|SetMaterial (Variables|Debug|GetStaticMeshComponent) 0 (Variables|Default|GetMat_Blue))
    (Variables|Default|SetIsRed false)
    (Variables|Default|SetIsRed_Int 0) ; 0 = false; = Blue
    (else
      (Rendering|Material|SetMaterial (Variables|Debug|GetStaticMeshComponent) 0 (Variables|Default|GetMat_Red))
      (Variables|Default|SetIsRed true)
      (Variables|Default|SetIsRed_Int 1) ; 1 = true; = Red
    )))