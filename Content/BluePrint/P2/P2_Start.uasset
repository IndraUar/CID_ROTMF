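; Start trigger for puzzle section P2 that saves a checkpoint and watches whether pressure plates share a color.
; On overlap, it writes its own transform as the player position to the P2_Save slot, creating the save if absent, then enables Tick.
; For puzzle index 1 or 2, Tick tallies matching BP_PressurePlate colors as plus or minus one.
; When all match, it prints "Same" and latches AllSame, ending the check.
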(event Collision|EventActorBeginOverlap
  (params (OtherActor :type Actor%20Object%20Reference))
  (Development|PrintString "Start P2")
  (if (Variables|Default|GetSaveExist)
    (bind _returnvalue (SaveGame|LoadGamefromSlot "P2_Save"))
    (bind _asp2_save (Utilities|Casting|CastToP2_Save _returnvalue))
    (Variables|/Game/BluePrint/Save_And_Load/P2_Save.P2_Save_C|SetP2_PlayerPosition _asp2_save (Transformation|GetActorTransform))
    (SaveGame|SaveGametoSlot _returnvalue "P2_Save")
    (else
      (bind _returnvalue_2 (SaveGame|CreateSaveGameObject "/Game/BluePrint/Save_And_Load/P2_Save.P2_Save_C"))
      (Variables|/Game/BluePrint/Save_And_Load/P2_Save.P2_Save_C|SetP2_PlayerPosition _returnvalue_2 (Transformation|GetActorTransform))
      (SaveGame|SaveGametoSlot _returnvalue_2 "P2_Save")))
  (Actor|Tick|SetActorTickEnabled true))

(event EventBeginPlay
  (Actor|Tick|SetActorTickEnabled false)
  (bind _returnvalue (SaveGame|DoesSaveGameExist "P2_Save"))
  (if _returnvalue
    (Variables|Default|SetSaveExist true)
    (bind _returnvalue_2 (SaveGame|LoadGamefromSlot "P2_Save"))
    (Utilities|Casting|CastToP2_Save _returnvalue_2)
    (else
      (Variables|Default|SetSaveExist false)
      (Development|PrintString "No Save(P2_Save)"))))

(event EventTick
  (params (DeltaSeconds :type Float%20%28single-precision%29))
  (Utilities|FlowControl|Sequence
    (:then_1
      (if (== (Variables|Default|GetPuzzleIndex) 1)
        (CallFunction|Index(2?)Color) ; later change to 1
      ))
    (:then_2
      (if (== (Variables|Default|GetPuzzleIndex) 2)
        (CallFunction|Index(2?)Color)))))

(fn ConstructionScript)

(fn Index(2?)Color
  (bind _outactors (Actor|GetAllActorsOfClass "/Game/BluePrint/P2/PressurePlate/BP_PressurePlate.BP_PressurePlate_C"))
  (if (not (Variables|Default|GetAllSame))
    (for _array_element _outactors
      (if (== (Variables|/Game/BluePrint/P2/PressurePlate/BP_PressurePlate.BP_PressurePlate_C|GetPlate_Puzzle_Index _array_element) (Variables|Default|GetPuzzleIndex))
        (Variables|Default|SetAmountOfPlate (+ (Variables|Default|GetAmountOfPlate) 1))
        (if (== (Variables|/Game/BluePrint/P2/PressurePlate/BP_PressurePlate.BP_PressurePlate_C|GetColorInt _array_element) 0) ; true = blue; false = red
          (Variables|Default|SetTotalColorInt (- (Variables|Default|GetTotalColorInt) 1))
          (else
            (Variables|Default|SetTotalColorInt (+ (Variables|Default|GetTotalColorInt) 1))))))
    (if (< (Variables|Default|GetTotalColorInt) 0)
      (if (== (Variables|Default|GetAmountOfPlate) (* (Variables|Default|GetTotalColorInt) -1))
        (Development|PrintString "Same" :!label _label)
        (Variables|Default|SetAllSame true)
        (else
          (Variables|Default|SetAmountOfPlate 0 :!label _label_2)
          (Variables|Default|SetTotalColorInt 0)))
      (elif (== (Variables|Default|GetAmountOfPlate) (Variables|Default|GetTotalColorInt))
        (goto _label)
        (else
          (goto _label_2))))))