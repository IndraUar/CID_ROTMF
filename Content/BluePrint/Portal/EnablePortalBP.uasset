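; EnablePortalBP keeps an entrance and exit portal pair disabled until the collected shard count equals the total.
; BeginPlay hides both referenced portals, turns off their collision and stops their root component tick.
; Tick compares CollectedShard to TotalShred and, through a DoOnce, restores visibility, collision and root ticking a single time when they match.
; The shard counter is only read here, with no logic in this graph to update it.
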(event EventTick
  (params (DeltaSeconds :type Float%20%28single-precision%29))
  (bind _portal_enterance (Variables|Default|GetPortal_Enterance))
  (if (== (Variables|Default|GetCollectedShard) (Variables|Default|GetTotalShred))
    (Utilities|FlowControl|DoOnce false
      (:Completed
        (Rendering|SetVisibility (Variables|/Script/Engine.Actor|GetRootComponent (Variables|Default|GetPortal_Exit)) true true)
        (Collision|SetActorEnableCollision _portal_enterance true)
        (Components|Tick|SetComponentTickEnabled (Variables|/Script/Engine.Actor|GetRootComponent _portal_enterance) true)))))

(event EventBeginPlay
  (bind _portal_enterance (Variables|Default|GetPortal_Enterance))
  (Rendering|SetVisibility (Variables|/Script/Engine.Actor|GetRootComponent (Variables|Default|GetPortal_Exit)) false true)
  (Collision|SetActorEnableCollision _portal_enterance false)
  (Components|Tick|SetComponentTickEnabled (Variables|/Script/Engine.Actor|GetRootComponent _portal_enterance) false))

(fn ConstructionScript)