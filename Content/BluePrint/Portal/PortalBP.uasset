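; PortalBP is a paired portal actor that teleports the third-person character to its linked partner.
; On hit by that character it plays a sound, then searches all PortalBP actors for one with the same PortalIndex and the opposite Enterance flag, so travel works both ways.
; It moves the character to the partner's ExitReference location and spawns a confetti Niagara effect there.
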(event Collision|EventHit
  (params (MyComp :type Primitive%20Component%20Object%20Reference) (Other :type Actor%20Object%20Reference) (OtherComp :type Primitive%20Component%20Object%20Reference) (bSelfMoved :type Boolean) (HitLocation :type Vector :default "0, 0, 0") (HitNormal :type Vector :default "0, 0, 0") (NormalImpulse :type Vector :default "0, 0, 0") (Hit :type Hit%20Result%20Structure%20%28by%20ref%29))
  (bind _asbp_third_person_character (Utilities|Casting|CastToBP_ThirdPersonCharacter Other))
  (Audio|PlaySound2D "/Engine/VREditor/Sounds/UI/Enter_Simulate.Enter_Simulate" 1.0 1.0 0.0 0 0)
  (if (Variables|Default|GetEnterance)
    (bind _outactors (Actor|GetAllActorsOfClass "PortalBP_C"))
    (bind _array_element (Utilities|Array|ForEachLoopwithBreak _outactors :!label _label)
      (:LoopBody
        (if (and (== (Variables|PortalBP_C|GetPortal%20Index _array_element) (Variables|Default|GetPortal%20Index)) (not (Variables|PortalBP_C|GetEnterance _array_element)))
          (goto _label Break)))
      (:Completed
        (Transformation|SetActorLocation _asbp_third_person_character (Transformation|GetWorldLocation (Variables|PortalBP_C|GetExit%20Reference _array_element)) false false)
        (Niagara|SpawnSystematLocation "/Game/VisualFX/VFX_Confetti/VFX_Confetti.VFX_Confetti" (Transformation|GetWorldLocation (Variables|PortalBP_C|GetExit%20Reference _array_element)))))
    (else
      (bind _outactors_2 (Actor|GetAllActorsOfClass "PortalBP_C"))
      (bind _array_element_2 (Utilities|Array|ForEachLoopwithBreak _outactors_2 :!label _label_2)
        (:LoopBody
          (if (and (== (Variables|PortalBP_C|GetPortal%20Index _array_element_2) (Variables|Default|GetPortal%20Index)) (and (not (Variables|Default|GetEnterance)) (Variables|PortalBP_C|GetEnterance _array_element_2)))
            (goto _label_2 Break)))
        (:Completed
          (Transformation|SetActorLocation _asbp_third_person_character (Transformation|GetWorldLocation (Variables|PortalBP_C|GetExit%20Reference _array_element_2)) false false)
          (Niagara|SpawnSystematLocation "/Game/VisualFX/VFX_Confetti/VFX_Confetti.VFX_Confetti" (Transformation|GetWorldLocation (Variables|PortalBP_C|GetExit%20Reference _array_element_2))))))))

(fn ConstructionScript)