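; Lever switch actor that drives two Door_Blue actors when its handle crosses the level position.
; Tick converts the handle's world rotation into actor-local space and treats negative pitch as On.
; Whenever that state flips, in either direction, it calls Lift on the ToLift door and Lower on the ToLower door.
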(event EventBeginPlay)

(event Collision|EventActorBeginOverlap
  (params (OtherActor :type Actor%20Object%20Reference)))

(event EventTick
  (params (DeltaSeconds :type Float%20%28single-precision%29))
  (bind _returnvalue (Transformation|GetActorTransform))
  (bind _handle (Variables|Default|GetHandle))
  (bind _returnvalue_2 (Transformation|GetWorldRotation _handle))
  (bind _returnvalue_3 (Math|Transform|InverseTransformRotation _returnvalue _returnvalue_2))
  (bind _returnvalue_4 (< (.pitch _returnvalue_3) 0.0))
  (if (!= (Variables|Default|GetOn) _returnvalue_4)
    (Variables|Default|SetOn _returnvalue_4)
    (Utilities|FlowControl|Sequence
      (:then_0
        (bind _asswitcher_door (Utilities|Casting|CastToDoor_Blue (Variables|Default|GetToLift)))
        (Default|Lift _asswitcher_door))
      (:then_1
        (bind _asswitcher_door_2 (Utilities|Casting|CastToDoor_Blue (Variables|Default|GetToLower)))
        (Default|Lower _asswitcher_door_2)))))

(fn ConstructionScript)