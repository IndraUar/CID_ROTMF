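; SwitcherDoor is a door actor in the Pull_Lever folder that shifts vertically by a set Distance when toggled.
; Lift and Lower both flip the Lifted flag, print debug state and instantly offset the whole actor in Z, with opposite directions.
; An eased MoveComponentTo of the Door component, timed by Speed, sits unconnected in the event graph, whose events are empty.
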(event EventBeginPlay)

(event Collision|EventActorBeginOverlap
  (params (OtherActor :type Actor%20Object%20Reference)))

(event EventTick
  (params (DeltaSeconds :type Float%20%28single-precision%29)))

(fn ConstructionScript)

(fn Lift
  (if (Variables|Default|GetLifted)
    (Development|PrintString "Off (Down)")
    (Variables|Default|SetLifted false)
    (Transformation|AddActorWorldOffset (Math|Vector|MakeVector 0.0 0.0 (* (Variables|Default|GetDistance) -1.0)))
    (else
      (Development|PrintString "On (Up)")
      (Variables|Default|SetLifted true)
      (Transformation|AddActorWorldOffset (Math|Vector|MakeVector 0.0 0.0 (Variables|Default|GetDistance))))))

(fn Lower
  (if (Variables|Default|GetLifted)
    (Development|PrintString "Off")
    (Variables|Default|SetLifted false)
    (Transformation|AddActorWorldOffset (Math|Vector|MakeVector 0.0 0.0 (Variables|Default|GetDistance)))
    (else
      (Development|PrintString "On")
      (Variables|Default|SetLifted true)
      (Transformation|AddActorWorldOffset (Math|Vector|MakeVector 0.0 0.0 (* (Variables|Default|GetDistance) -1.0))))))