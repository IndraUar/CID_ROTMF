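; Actor component that lets its owning Character grab and push or pull objects in the world.
; BeginPush attaches the character to the object, stops orient-to-movement and enables tick; EndPush reverses this.
; Tick moves the object with a swept offset built from ForwardMove, RightMove, PushSpeed and the character's facing vectors, carrying the attached character along.
; Tick's four yaw-direction branches all apply the same offset.
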(event EventBeginPlay
  (Components|Tick|SetComponentTickEnabled false)
  (bind _ascharacter (Utilities|Casting|CastToCharacter (Components|GetOwner)))
  (Variables|Default|SetCharacter _ascharacter))

(event EventTick
  (params (DeltaSeconds :type Float%20%28single-precision%29))
  (Variables|Default|SetCurrentActorZRotation (.yaw (Transformation|GetActorRotation (Variables|Default|GetCharacter))))
  ;[1 1 1] Up
  (if (and (>= (Variables|Default|GetCurrentActorZRotation) -15.0) (< (Variables|Default|GetCurrentActorZRotation) 8e+01))
    (bind _currentpushableobject (Variables|Default|GetCurrentPushableObject)
      (:then
        (Transformation|AddActorWorldOffset _currentpushableobject (CallFunction|GetDeltaLocation DeltaSeconds (Variables|Default|GetForwardMove) (Variables|Default|GetRightMove)) true))
      (:else))
    (else
      ;[1 1 1] Right
      (if (and (>= (Variables|Default|GetCurrentActorZRotation) 8e+01) (< (Variables|Default|GetCurrentActorZRotation) 1.4e+02))
        (bind _currentpushableobject_2 (Variables|Default|GetCurrentPushableObject)
          (:then
            (Transformation|AddActorWorldOffset _currentpushableobject_2 (CallFunction|GetDeltaLocation DeltaSeconds (Variables|Default|GetForwardMove) (Variables|Default|GetRightMove)) true))
          (:else))
        (else
          ;[1 1 1] Left
          (if (and (>= (Variables|Default|GetCurrentActorZRotation) -1.3e+02) (< (Variables|Default|GetCurrentActorZRotation) 0.0))
            (bind _currentpushableobject_3 (Variables|Default|GetCurrentPushableObject)
              (:then
                (Transformation|AddActorWorldOffset _currentpushableobject_3 (CallFunction|GetDeltaLocation DeltaSeconds (Variables|Default|GetForwardMove) (Variables|Default|GetRightMove)) true))
              (:else))
            (else
              ;[1 1 1] Down
              (if (and (>= (Variables|Default|GetCurrentActorZRotation) -1.8e+02) (< (Variables|Default|GetCurrentActorZRotation) 1.8e+02))
                (bind _currentpushableobject_4 (Variables|Default|GetCurrentPushableObject)
                  (:then
                    (Transformation|AddActorWorldOffset _currentpushableobject_4 (CallFunction|GetDeltaLocation DeltaSeconds (Variables|Default|GetForwardMove) (Variables|Default|GetRightMove)) true))
                  (:else))))))))))

(fn BeginPush
  (params (PushableObject :type BP%20Pushable%20Object%20Object%20Reference))
  (bind _character (Variables|Default|GetCharacter))
  (Variables|Default|GetCurrentPushableObject
    (:then)
    (:else
      (bind _output_get (Variables|Default|SetCurrentPushableObject PushableObject))
      (Transformation|AttachActorToActor _character _output_get "None" "KeepWorld" "KeepWorld" "KeepWorld" true)
      (Variables|/Script/Engine.CharacterMovementComponent|SetbOrientRotationToMovement (Variables|/Script/Engine.Character|GetCharacterMovement _character) false)
      (Components|Tick|SetComponentTickEnabled true))))

(fn EndPush
  (bind _character (Variables|Default|GetCharacter))
  (Variables|Default|GetCurrentPushableObject
    (:then
      (Variables|Default|SetCurrentPushableObject 0)
      (Variables|Default|SetIsMovingAnObject false)
      (Transformation|DetachFromActor _character "KeepWorld" "KeepWorld" "KeepWorld")
      (Variables|/Script/Engine.CharacterMovementComponent|SetbOrientRotationToMovement (Variables|/Script/Engine.Character|GetCharacterMovement _character) true)
      (Components|Tick|SetComponentTickEnabled false))
    (:else)))

(fn IsHoldingObject
  (return (Utilities|IsValid (Variables|Default|GetCurrentPushableObject))))

(fn GetDeltaLocation
  (params (DeltaSecond :type Float%20%28double-precision%29) (ForwardMove :type Float%20%28double-precision%29) (RightMove :type Float%20%28double-precision%29))
  (Variables|Default|SetIsMovingAnObject (or (!= ForwardMove 0.0) (!= RightMove 0.0)))
  (return (+ (* (* (Transformation|GetActorForwardVector (Variables|Default|GetCharacter)) ForwardMove) (* DeltaSecond (Variables|Default|GetPushSpeed))) (* (* (Transformation|GetActorRightVector (Variables|Default|GetCharacter)) RightMove) (* (Variables|Default|GetPushSpeed) DeltaSecond)))))