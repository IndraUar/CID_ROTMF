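; Load_P1 is an unfinished loader for the Artifact_P1 save slot, triggered by the P key.
; P loads the slot if it exists or prints a missing-save message, but the loaded object is not applied.
; BeginPlay calls GetActorOfClass without using the result.
; Disconnected nodes sketch an artifact check, casts to the character and lever switcher, a transform restore and a main-door lever restore, none of which run.
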(event EventBeginPlay
  (Actor|GetActorOfClass 0))

(event Input|KeyboardEvents|O
  (params (Key :type Key%20Structure :default "None")))

(event Input|KeyboardEvents|P
  (params (Key :type Key%20Structure :default "None"))
  (:Pressed
    (SaveGame|DoesSaveGameExist "Artifact_P1")
    (if true
      (SaveGame|LoadGamefromSlot "Artifact_P1")
      (else
        (Development|PrintString "No Saved File")))))

(fn ConstructionScript)